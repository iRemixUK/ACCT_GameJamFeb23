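; Base enemy Blueprint that supplies patrol and chase movement functions and takes damage from projectiles.
; On BeginPlay it caches every BP_PatrolLocation, and MoveToRandomLocation walks straight to a random one, using a squared XY distance check for arrival.
; MoveToPlayer flags the player as seen and steps toward them.
; Collider overlaps with BP_ProjectileAttack apply fixed damage and print Life; neither movement function is called in these graphs.
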(event OnComponentBeginOverlap(Collider)
  (params (OverlappedComponent :type Primitive%20Component%20Object%20Reference) (OtherActor :type Actor%20Object%20Reference) (OtherComp :type Primitive%20Component%20Object%20Reference) (OtherBodyIndex :type Integer) (bFromSweep :type Boolean) (SweepResult :type Hit%20Result%20Structure%20%28by%20ref%29))
  ;[1 1 1] If collider of enemy is hit by bullet enemy takes damage
  (Utilities|Casting|CastToBP_ProjectileAttack OtherActor)
  (Class|CustomBasePawn|Damage 25)
  (Development|PrintString (Utilities|String|ToString(Integer) (Variables|Default|GetLife))))

(event EventBeginPlay
  (|CallParentFunction)
  (bind _outactors (Actor|GetAllActorsOfClass "/Game/Blueprints/BP_PatrolLocation.BP_PatrolLocation_C"))
  (Variables|Default|SetPatrolLocations _outactors))

(event Collision|EventActorBeginOverlap
  (params (OtherActor :type Actor%20Object%20Reference))
  (|CallParentFunction OtherActor) ; This node is disabled and will not be called.\nDrag off pins to build functionality.
)

(event EventTick
  (params (DeltaSeconds :type Float%20%28single-precision%29))
  (|CallParentFunction DeltaSeconds) ; This node is disabled and will not be called.\nDrag off pins to build functionality.
)

(fn ConstructionScript
  (|CallParentFunction))

(fn MovetoPlayer
  (params (Player :type Pawn%20Object%20Reference))
  (Variables|Default|SetCanSeePlayer true)
  (Class|CustomBasePawn|Move (Math|Vector|GetUnitDirection(Vector) (Transformation|GetActorLocation) (Transformation|GetActorLocation Player)) (Utilities|Time|GetWorldDeltaSeconds)))

(fn MovetoRandomLocation
  (bind _returnvalue (Transformation|GetActorLocation))
  (if (Variables|Default|GetisMoving)
    (Variables|Default|SetMovementSpeed 5e+02)
    (Class|CustomBasePawn|Move (Variables|Default|GetDirection) (Utilities|Time|GetWorldDeltaSeconds))
    (if (<= (+ (Math|Float|Square (- (.x (Transformation|GetActorLocation (Variables|Default|GetRandomActor))) (.x _returnvalue))) (Math|Float|Square (- (.y (Transformation|GetActorLocation (Variables|Default|GetRandomActor))) (.y _returnvalue)))) 1e+02)
      (Variables|Default|SetMovementSpeed 0.0)
      (Variables|Default|SetisMoving false))
    (else
      (Variables|Default|SetMovementSpeed 0.0)
      (bind _output_get (Variables|Default|SetRandomActor (.OutItem (Utilities|Array|Random (Variables|Default|GetPatrolLocations)))))
      (Variables|Default|SetDirection (Math|Vector|GetUnitDirection(Vector) (Transformation|GetActorLocation) (Transformation|GetActorLocation _output_get)))
      (Variables|Default|SetisMoving true))))