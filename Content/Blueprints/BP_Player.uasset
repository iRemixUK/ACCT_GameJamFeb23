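; Player actor that moves, jumps, fires directional projectiles and respawns at checkpoints.
; Forward and right axes feed Move, while jumping applies an upward capsule impulse, locked by a Tick countdown rather than a ground check.
; Right mouse spawns BP_ProjectileAttack rotated to match CompassDirection, passing it DamagePower.
; Die plays particles, hides the player and makes the capsule static, then after a delay restores it at the last checkpoint transform.
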(event EventBeginPlay
  (|CallParentFunction) ; This node is disabled and will not be called.\nDrag off pins to build functionality.
)

(event Collision|EventActorBeginOverlap
  (params (OtherActor :type Actor%20Object%20Reference))
  (|CallParentFunction OtherActor) ; This node is disabled and will not be called.\nDrag off pins to build functionality.
)

(event EventTick
  (params (DeltaSeconds :type Float%20%28single-precision%29))
  (|CallParentFunction DeltaSeconds)
  (bind _output_get (Variables|Default|SettimerVariable (Math|Float|Max(Float) (- (Variables|Default|GettimerVariable) DeltaSeconds) 0.0)))
  (Math|Float|CompareFloat _output_get 0.0
    (:==
      (Variables|Default|SetbIsJumping false))))

(event EventDie
  (bind _returnvalue (Transformation|GetActorTransform))
  (bind (_location _rotation _scale) (Math|Transform|BreakTransform _returnvalue))
  (Niagara|SpawnSystematLocation (Variables|Default|GetDieParticles) _location _rotation _scale)
  (Rendering|SetActorHiddenInGame true)
  (Transformation|SetMobility (Variables|Default|GetCapsuleCollider) "Static")
  (Utilities|FlowControl|Delay 3.0)
  (Transformation|SetMobility (Variables|Default|GetCapsuleCollider) "Movable")
  (Transformation|SetActorTransform (Variables|Default|GetLastCheckpointTransfrom))
  (Rendering|SetActorHiddenInGame false))

(event EventAttack
  (bind _returnvalue (Transformation|GetActorTransform))
  (bind _returnvalue_2 (Transformation|GetActorTransform))
  (bind _returnvalue_3 (Transformation|GetActorTransform))
  (bind _returnvalue_4 (Transformation|GetActorTransform))
  (bind (_location _rotation _scale) (Math|Transform|BreakTransform _returnvalue))
  (bind (_location_2 _rotation_2 _scale_2) (Math|Transform|BreakTransform _returnvalue_2))
  (bind (_location_3 _rotation_3 _scale_3) (Math|Transform|BreakTransform _returnvalue_3))
  (bind (_location_4 _rotation_4 _scale_4) (Math|Transform|BreakTransform _returnvalue_4))
  (switch Utilities|FlowControl|Switch|SwitchonEDirection (Variables|Default|GetCompassDirection)
    (:North
      (bind _returnvalue_5 (Game|SpawnActorfromClass "/Game/Blueprints/BP_ProjectileAttack.BP_ProjectileAttack_C" (Math|Transform|MakeTransform _location "0, 0, 0" _scale) "Undefined" 0 0))
      (Variables|/Game/Blueprints/BP_ProjectileAttack.BP_ProjectileAttack_C|SetDamage _returnvalue_5 (Variables|Default|GetDamagePower)))
    (:South
      (bind _returnvalue_6 (Game|SpawnActorfromClass "/Game/Blueprints/BP_ProjectileAttack.BP_ProjectileAttack_C" (Math|Transform|MakeTransform _location_4 "0,180.000000, 0" _scale_4) "Undefined" 0 0))
      (Variables|/Game/Blueprints/BP_ProjectileAttack.BP_ProjectileAttack_C|SetDamage _returnvalue_6 (Variables|Default|GetDamagePower)))
    (:East
      (bind _returnvalue_7 (Game|SpawnActorfromClass "/Game/Blueprints/BP_ProjectileAttack.BP_ProjectileAttack_C" (Math|Transform|MakeTransform _location_3 "0,90.000000, 0" _scale_3) "Undefined" 0 0))
      (Variables|/Game/Blueprints/BP_ProjectileAttack.BP_ProjectileAttack_C|SetDamage _returnvalue_7 (Variables|Default|GetDamagePower)))
    (:West
      (bind _returnvalue_8 (Game|SpawnActorfromClass "/Game/Blueprints/BP_ProjectileAttack.BP_ProjectileAttack_C" (Math|Transform|MakeTransform _location_2 "0,270.000000, 0" _scale_2) "Undefined" 0 0))
      (Variables|/Game/Blueprints/BP_ProjectileAttack.BP_ProjectileAttack_C|SetDamage _returnvalue_8 (Variables|Default|GetDamagePower)))))

(event Input|ActionEvents|InputActionJump
  (params (Key :type Key%20Structure :default "None"))
  (:Pressed
    (if (not (Variables|Default|GetbIsJumping))
      (Physics|AddImpulse (Variables|Default|GetCapsuleCollider) "0, 0,500.000000" "None" true)
      (Variables|Default|SetbIsJumping true)
      (Variables|Default|SettimerVariable 1.0))))

(event Input|AxisEvents|InputAxisForward
  (params (AxisValue :type Float%20%28single-precision%29))
  ;[1 1 1] Characters Movement
  (Class|CustomBasePawn|Move (Math|Vector|MakeVector (Input|AxisValues|GetForward) (Input|AxisValues|GetRight) 0.0) (Utilities|Time|GetWorldDeltaSeconds)))

(event Input|AxisEvents|InputAxisRight
  (params (AxisValue :type Float%20%28single-precision%29))
  ;[1 1 1] Characters Movement
  (Class|CustomBasePawn|Move (Math|Vector|MakeVector (Input|AxisValues|GetForward) (Input|AxisValues|GetRight) 0.0) (Utilities|Time|GetWorldDeltaSeconds)))

(event Input|MouseEvents|RightMouseButton
  (params (Key :type Key%20Structure :default "None"))
  (:Pressed
    (Class|CustomBasePawn|Attack)))

(fn ConstructionScript
  (|CallParentFunction))