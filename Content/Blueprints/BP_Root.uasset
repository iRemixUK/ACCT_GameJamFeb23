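; BP_Root is a spline-based actor that builds a root shape out of repeated mesh segments.
; The construction script creates one dynamic material instance, then adds a spline mesh component for each segment of RootSpline.
; Each component bends RootSegmentMesh along X using that segment's local positions and tangents, shares the material and uses physics-only collision.
; It has no runtime logic.
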(event EventBeginPlay)

(event Collision|EventActorBeginOverlap
  (params (OtherActor :type Actor%20Object%20Reference)))

(event EventTick
  (params (DeltaSeconds :type Float%20%28single-precision%29)))

(fn ConstructionScript
  (bind _rootspline (Variables|Default|GetRootSpline))
  (bind _returnvalue (Rendering|Material|CreateDynamicMaterialInstance (Variables|Default|GetMaterialBase) "None" "None" :!class /Script/Engine.KismetMaterialLibrary))
  (Variables|Default|SetMaterialInstance _returnvalue)
  (for _index (range 0 (+ (Class|SplineComponent|GetNumberOfSplineSegments _rootspline) -1))
    (bind _returnvalue_2 (AddComponent|AddSplineMeshComponent false))
    (Collision|SetCollisionEnabled _returnvalue_2 "PhysicsOnly")
    (SplineMesh|SetForwardAxis _returnvalue_2 "X" true)
    (Components|StaticMesh|SetStaticMesh _returnvalue_2 (Variables|Default|GetRootSegmentMesh))
    (Rendering|Material|SetMaterial _returnvalue_2 0 (Variables|Default|GetMaterialInstance))
    (SplineMesh|SetStartandEnd _returnvalue_2 (Spline|GetLocationatSplinePoint _rootspline _index "Local") (Spline|GetTangentatSplinePoint _rootspline _index "Local") (Spline|GetLocationatSplinePoint _rootspline (+ _index 1) "Local") (Spline|GetTangentatSplinePoint _rootspline (+ _index 1) "Local") true :!class /Script/Engine.SplineMeshComponent)))