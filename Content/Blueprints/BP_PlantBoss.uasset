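; BP_PlantBoss is a plant boss that launches projectiles when it sees a pawn.
; Its PawnSensing OnSeePawn event runs a one-second Delay, then spawns a BP_PlantProjectile above the boss's location.
; The Delay also throttles firing, since sightings that arrive while it counts down are ignored.
; The seen pawn is not used, and no aim rotation is set on the spawn.
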(event OnSeePawn(PawnSensing)
  (params (Pawn :type Pawn%20Object%20Reference))
  (Utilities|FlowControl|Delay 1.0)
  (Game|SpawnActorfromClass "/Game/Blueprints/BP_PlantProjectile.BP_PlantProjectile_C" (Math|Transform|MakeTransform (+ (Transformation|GetActorLocation) "0,0.000000,200.000000") "0, 0, 0" "1.000000,1.000000,1.000000") "Undefined" 0 0))

(event EventBeginPlay
  (|CallParentFunction) ; This node is disabled and will not be called.\nDrag off pins to build functionality.
)

(event Collision|EventActorBeginOverlap
  (params (OtherActor :type Actor%20Object%20Reference))
  (|CallParentFunction OtherActor) ; This node is disabled and will not be called.\nDrag off pins to build functionality.
)

(event EventTick
  (params (DeltaSeconds :type Float%20%28single-precision%29))
  (|CallParentFunction DeltaSeconds) ; This node is disabled and will not be called.\nDrag off pins to build functionality.
)

(fn ConstructionScript
  (|CallParentFunction))