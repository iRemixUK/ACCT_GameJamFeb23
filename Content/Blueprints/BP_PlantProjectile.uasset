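; BP_PlantProjectile is a projectile that aims itself at the player pawn when it spawns.
; On BeginPlay it predicts where the player will be by scaling their velocity by distance over projectile speed, targeting slightly below the pawn's location.
; SuggestProjectileVelocity turns that lead point into an arcing toss velocity, which drives the ProjectileMovement component with rotation following velocity.
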(event EventBeginPlay
  (bind _returnvalue (Game|Player|GetPlayerPawn 0))
  (bind _projectilemovement (Variables|Default|GetProjectileMovement))
  (bind _tossvelocity (Class|GameplayStatics|BlueprintSuggestProjectileVelocity (Transformation|GetActorLocation) (+ (- (Transformation|GetActorLocation _returnvalue) "0,0,50.000000") (* (/ (Transformation|GetDistanceTo _returnvalue) (Variables|Default|GetProjectileSpeed)) (Transformation|GetVelocity _returnvalue))) (Variables|Default|GetProjectileSpeed) 0.0 "DoNotTrace" 0.0 false false))
  (Variables|/Script/Engine.MovementComponent|SetVelocity _projectilemovement _tossvelocity)
  (Variables|/Script/Engine.ProjectileMovementComponent|SetbRotationFollowsVelocity _projectilemovement true))

(fn ConstructionScript)