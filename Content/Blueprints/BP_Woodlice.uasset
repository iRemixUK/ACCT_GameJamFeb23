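; Woodlice enemy that chases the player and deals damage on contact.
; Each tick it compares player distance to vision range to enable movement, and to pursuit range to trigger a brief halt, then a speed burst ended by an accumulated timer.
; Colliding while mobile with anything but another woodlouse pauses it briefly, damaging the player if hit.
; Overlap-based detection is left disconnected in favor of the distance checks.
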(event OnComponentBeginOverlap(EnemySeeCollisionDetection)
  (params (OverlappedComponent :type Primitive%20Component%20Object%20Reference) (OtherActor :type Actor%20Object%20Reference) (OtherComp :type Primitive%20Component%20Object%20Reference) (OtherBodyIndex :type Integer) (bFromSweep :type Boolean) (SweepResult :type Hit%20Result%20Structure%20%28by%20ref%29)))

(event OnComponentEndOverlap(EnemySeeCollisionDetection)
  (params (OverlappedComponent :type Primitive%20Component%20Object%20Reference) (OtherActor :type Actor%20Object%20Reference) (OtherComp :type Primitive%20Component%20Object%20Reference) (OtherBodyIndex :type Integer)))

(event OnComponentBeginOverlap(EnemyAttackCollisionDetection)
  (params (OverlappedComponent :type Primitive%20Component%20Object%20Reference) (OtherActor :type Actor%20Object%20Reference) (OtherComp :type Primitive%20Component%20Object%20Reference) (OtherBodyIndex :type Integer) (bFromSweep :type Boolean) (SweepResult :type Hit%20Result%20Structure%20%28by%20ref%29)))

(event EventTick
  (params (DeltaSeconds :type Float%20%28single-precision%29))
  (|CallParentFunction DeltaSeconds)
  (Utilities|FlowControl|Sequence
    (:then_0
      (if (Variables|Default|GetCanMove)
        (CallFunction|MovetoPlayer (Game|Player|GetPlayerPawn 0))
        (if (Variables|Default|GetInPursuit)
          (CallFunction|StartTimer)
          (if (>= (Variables|Default|GetTimer) 5.0)
            (Development|PrintString "timer finish")
            (Variables|Default|SetTimer 0.0)
            (Variables|Default|SetInPursuit false)
            (Variables|Default|SetMovementSpeed (Variables|Default|GetDefaultMoveSpeed))))))
    (:then_1
      (if (<= (Math|Vector|Distance(Vector) (Transformation|GetActorLocation (Game|Player|GetPlayerPawn 0)) (Transformation|GetActorLocation)) (Variables|Default|GetVisionRange))
        (if (not (Variables|Default|GetIsAttacking))
          (Variables|Default|SetCanSeePlayer true)
          (Variables|Default|SetCanMove true))
        (else
          (Variables|Default|SetCanSeePlayer false)
          (Variables|Default|SetCanMove false))))
    (:then_2
      (if (<= (Math|Vector|Distance(Vector) (Transformation|GetActorLocation (Game|Player|GetPlayerPawn 0)) (Transformation|GetActorLocation)) (Variables|Default|GetPursuitRange))
        (if (Variables|Default|GetCanMove)
          (if (not (Variables|Default|GetInPursuit))
            (Variables|Default|SetInPursuit true)
            (if (not (Variables|Default|GetIsAttacking))
              (Development|PrintString "pursuit")
              (Variables|Default|SetMovementSpeed 0.0)
              (Utilities|FlowControl|Delay 0.5)
              (Variables|Default|SetMovementSpeed (Variables|Default|GetPursuitMoveSpeed)))))))))

(event EventOnColliderEnter
  (params (OverlappedComp :type Primitive%20Component%20Object%20Reference) (OtherActor :type Actor%20Object%20Reference) (OtherComp :type Primitive%20Component%20Object%20Reference) (OtherBodyIndex :type Integer) (bFromSweep :type Boolean) (SweepResult :type Hit%20Result%20Structure%20%28by%20ref%29))
  (if (Variables|Default|GetCanMove)
    (Utilities|Casting|CastToBP_Woodlice OtherActor
      (:CastFailed
        (bind _asbp_player (Utilities|Casting|CastToBP_Player OtherActor)
          (:then
            (Variables|Default|SetIsAttacking true)
            (Class|CustomBasePawn|Damage _asbp_player (Variables|Default|GetDamagePower)))
          (:CastFailed
            _))
        (Development|PrintString "player attack")
        (Variables|Default|SetMovementSpeed 0.0)
        (Variables|Default|SetCanMove false)
        (Utilities|FlowControl|Delay 1.0)
        (Variables|Default|SetMovementSpeed (Variables|Default|GetDefaultMoveSpeed))
        (Variables|Default|SetIsAttacking false)
        (Variables|Default|SetCanMove true)))))

(fn ConstructionScript
  (|CallParentFunction))

(fn StartTimer
  (bind _output_get (Variables|Default|SetTimer (+ (stale _output_get) (Utilities|Time|GetWorldDeltaSeconds)))))