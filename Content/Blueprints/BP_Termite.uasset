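; BP_Termite is an enemy or creature that wanders randomly and moves toward the player when it sees one.
; Tick calls MoveToRandomLocation whenever CanSeePlayer is false.
; PawnSensing sightings of BP_Player call MoveToPlayer, then a retriggerable delay of twice the sensing interval clears CanSeePlayer once sightings stop.
; The movement functions, and wherever CanSeePlayer becomes true, are not shown in these graphs.
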(event OnSeePawn(PawnSensing)
  (params (Pawn :type Pawn%20Object%20Reference))
  (bind _asbp_player (Utilities|Casting|CastToBP_Player Pawn))
  (CallFunction|MovetoPlayer _asbp_player)
  (Utilities|FlowControl|RetriggerableDelay (* (Variables|/Script/AIModule.PawnSensingComponent|GetSensingInterval (Variables|Default|GetPawnSensing)) 2.0))
  (Variables|Default|SetCanSeePlayer false))

(event EventBeginPlay
  (|CallParentFunction) ; This node is disabled and will not be called.\nDrag off pins to build functionality.
)

(event Collision|EventActorBeginOverlap
  (params (OtherActor :type Actor%20Object%20Reference))
  (|CallParentFunction OtherActor) ; This node is disabled and will not be called.\nDrag off pins to build functionality.
)

(event EventTick
  (params (DeltaSeconds :type Float%20%28single-precision%29))
  (|CallParentFunction DeltaSeconds)
  (if (not (Variables|Default|GetCanSeePlayer))
    (CallFunction|MovetoRandomLocation)))

(fn ConstructionScript
  (|CallParentFunction))