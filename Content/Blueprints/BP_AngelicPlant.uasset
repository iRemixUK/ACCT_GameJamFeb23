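; BP_AngelicPlant is a damageable plant actor linked to a RootParent.
; With a valid RootParent, it marks that parent Relevant on BeginPlay and hides its capsule's child components until Activate reveals them, keeping both colliders invisible.
; Damage only passes to the parent class while PlaneFront is visible, and Tick calls Move with zero DeltaTime.
; On death it clears Relevant and calls RootsEnable on RootParent before the inherited Die.
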(event EventBeginPlay
  (bind _rootparent (Variables|Default|GetRootParent))
  (|CallParentFunction)
  (Utilities|IsValid _rootparent
    (:Is%20Valid
      (Variables|/Game/Blueprints/BP_Root.BP_Root_C|SetRelevant _rootparent true)
      (Rendering|SetVisibility (Variables|Default|GetCapsuleCollider) false true)
      (Rendering|SetVisibility (Variables|Default|GetCapsuleCollider) false false)
      (Rendering|SetVisibility (Variables|Default|GetCollider) false false))))

(event Collision|EventActorBeginOverlap
  (params (OtherActor :type Actor%20Object%20Reference))
  (|CallParentFunction OtherActor))

(event EventTick
  (params (DeltaSeconds :type Float%20%28single-precision%29))
  (|CallParentFunction DeltaSeconds)
  (Class|CustomBasePawn|Move (Math|Vector|MakeVector 1.0 0.0 0.0) 0.0))

(event EventDie
  (bind _rootparent (Variables|Default|GetRootParent))
  (Variables|/Game/Blueprints/BP_Root.BP_Root_C|SetRelevant _rootparent false)
  (Default|RootsEnable _rootparent)
  (|CallParentFunction))

(event EventDamage
  (params (ToDamage :type Integer))
  (if (Rendering|IsVisible (Variables|Default|GetPlaneFront))
    (|CallParentFunction ToDamage)))

(fn ConstructionScript
  (|CallParentFunction))

(fn Activate
  (Rendering|SetVisibility (Variables|Default|GetCapsuleCollider) true true)
  (Rendering|SetVisibility (Variables|Default|GetCapsuleCollider) false false)
  (Rendering|SetVisibility (Variables|Default|GetCollider) false false))