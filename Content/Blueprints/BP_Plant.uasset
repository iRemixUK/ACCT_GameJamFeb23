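; BP_Plant is a poisonous plant hazard with a Niagara gas effect, shown on BeginPlay.
; Tick checks the player pawn's distance against AttackRange, then after a short Delay calls Damage and prints a poison debug message.
; The Damage event is empty here, so no health changes in this graph.
; Overlap events are empty; the gas visibility toggles and looping DamageOverTime timer are disconnected.
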(event OnComponentBeginOverlap(Collider)
  (params (OverlappedComponent :type Primitive%20Component%20Object%20Reference) (OtherActor :type Actor%20Object%20Reference) (OtherComp :type Primitive%20Component%20Object%20Reference) (OtherBodyIndex :type Integer) (bFromSweep :type Boolean) (SweepResult :type Hit%20Result%20Structure%20%28by%20ref%29)))

(event OnComponentBeginOverlap(MakeGasVisible)
  (params (OverlappedComponent :type Primitive%20Component%20Object%20Reference) (OtherActor :type Actor%20Object%20Reference) (OtherComp :type Primitive%20Component%20Object%20Reference) (OtherBodyIndex :type Integer) (bFromSweep :type Boolean) (SweepResult :type Hit%20Result%20Structure%20%28by%20ref%29)))

(event OnComponentEndOverlap(MakeGasVisible)
  (params (OverlappedComponent :type Primitive%20Component%20Object%20Reference) (OtherActor :type Actor%20Object%20Reference) (OtherComp :type Primitive%20Component%20Object%20Reference) (OtherBodyIndex :type Integer)))

(event Custom|DamageOverTime
  (Class|CustomBasePawn|Damage 5))

(event EventBeginPlay
  (|CallParentFunction)
  (Rendering|SetVisibility (Variables|Default|GetNiagara) true false))

(event Collision|EventActorBeginOverlap
  (params (OtherActor :type Actor%20Object%20Reference))
  (|CallParentFunction OtherActor) ; This node is disabled and will not be called.\nDrag off pins to build functionality.
)

(event EventTick
  (params (DeltaSeconds :type Float%20%28single-precision%29))
  (|CallParentFunction DeltaSeconds)
  (if (<= (Math|Vector|Distance(Vector) (Transformation|GetActorLocation (Game|Player|GetPlayerPawn 0)) (Transformation|GetActorLocation)) (Variables|Default|GetAttackRange))
    (Utilities|FlowControl|Delay 0.2)
    (Class|CustomBasePawn|Damage 5)
    (Development|PrintString "poisoin damage")))

(event EventDamage
  (params (ToDamage :type Integer)))

(fn ConstructionScript
  (|CallParentFunction))